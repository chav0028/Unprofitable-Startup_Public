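; BP_NNTester is a test harness for a financial neural network that predicts scaled income from financial input data.
; On BeginPlay it creates the WidgetBP_NNTesting UI filled with that input and switches to UI-only input with a visible cursor.
; It then constructs a CFinancialNeuralNetwork from the model and scaling data path and triggers a first run through the widget.
; RunNNModel evaluates the current input, prints the result and returns it.
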(event `self.ReceiveBeginPlay`
  ;[1 1 1] Setup
  (`self.Set Testing UI`)
  (bind _returnvalue (`|GenericCreateObject` "/Script/UnprofitableStartup.CFinancialNeuralNetwork"))
  (set `self.m_netIncomeNN` _returnvalue)
  (`CFinancialNeuralNetwork.SetModel` (`self.m_netIncomeNN`) (`self.m_neuralNetworkModel`) (`self.m_scalingDataPath`))
  ;[1 1 1] Initial Run
  (`/Game/Blueprints/Testing/UI/WidgetBP_NNTesting.RunNNModel` (`self.m_testingUI`)))

(fn `RunNNModel`
  (returns (UnscaledNetIncome :type "Float (double-precision)"))
  (bind _returnvalue (`CFinancialNeuralNetwork.RunModel` (`self.m_netIncomeNN`) (`self.m_financialDataInput`)))
  (`KismetSystemLibrary.PrintString` (`KismetStringLibrary.Concat_StrStr` "Scaled Income of: " (`KismetStringLibrary.Conv_DoubleToString` _returnvalue)))
  (return _returnvalue))

(fn `Set Testing UI`
  (bind _returnvalue (`GameplayStatics.GetPlayerController` 0))
  (bind _returnvalue_2 (`|CreateWidget` "/Game/Blueprints/Testing/UI/WidgetBP_NNTesting.WidgetBP_NNTesting_C" _returnvalue self))
  (bind _output_get (set `self.m_testingUI` _returnvalue_2))
  (`/Game/Blueprints/Testing/UI/WidgetBP_NNTesting.SetTextBoxesValues` _output_get (`self.m_financialDataInput`))
  ;[1 1 1] Show UI
  (`UserWidget.AddToViewport` _output_get 0)
  (`WidgetBlueprintLibrary.SetInputMode_UIOnlyEx` _returnvalue _output_get "LockOnCapture")
  (`self.EnableInput` _returnvalue)
  (set `PlayerController.bShowMouseCursor` true _returnvalue))

(fn `UserConstructionScript`)