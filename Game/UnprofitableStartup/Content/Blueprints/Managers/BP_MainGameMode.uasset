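; Main game mode for a company management game that sets up the player's company and the in-game UI on BeginPlay.
; InitialiseCompany builds marketing and research expense objects from budgets and investment levels, then passes them to the company with starting financials.
; The company also receives a net-income neural network model with a scaling data file, plus balance limits on income change, handicap, stock value and marketing bonus.
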(event `self.ReceiveBeginPlay`
  (bind _returnvalue (`GameplayStatics.GetPlayerController` 0))
  (bind _returnvalue_2 (`self.GetPlayerCompany`))
  ;[1 1 1] Initialise the company
  (`/Engine/EditorBlueprintResources/StandardMacros.IsValid` _returnvalue_2
    (:`Is Valid`
      (`self.InitialiseCompany` _returnvalue_2)
      ;[1 1 1] Initialise the in-game UI
      (bind _returnvalue_3 (`|CreateWidget` "/Game/Blueprints/UI/Screens/WBP_InGameUI.WBP_InGameUI_C" _returnvalue))
      (`UserWidget.AddToViewport` _returnvalue_3 0)
      (set `PlayerController.bShowMouseCursor` true _returnvalue)
      ;[1 1 1] Limit Player input to UI only
      (`WidgetBlueprintLibrary.SetInputMode_GameAndUIEx` (`GameplayStatics.GetPlayerController` 0) _returnvalue_3))
    (:`Is Not Valid`
      (`KismetSystemLibrary.PrintString` "Invalid Player Company" false true (struct :`R` 1.0 :`A` 1.0)))))

(fn `InitialiseCompany`
  (params (aCompany :type "CCompany Object Reference"))
  (locals (marketingExpenses :type "CMonthlyExpenseInvestment Object Reference") (researchExpenses :type "CMonthlyExpenseInvestment Object Reference") (marketingInvestmentLevels :type "Array of SInvestmentLevel Structure") (researchInvestmentLevels :type "Array of SInvestmentLevel Structure") (marketingBudget :type Integer64 :default 25) (researchBudget :type Integer64 :default 25) (playerCompany :type "CCompany Object Reference"))
  (set `local.playerCompany` aCompany)
  ;[1 1 1] Initialise the expenses investment levels
  (bind _returnvalue (`|GenericCreateObject` "/Script/UnprofitableStartup.CMonthlyExpenseInvestment"))
  (bind _output_get (set `local.marketingExpenses` _returnvalue))
  (`CMonthlyExpenseInvestment.Initialise` _output_get (`local.marketingBudget`) (`local.marketingInvestmentLevels`))
  (bind _returnvalue_2 (`|GenericCreateObject` "/Script/UnprofitableStartup.CMonthlyExpenseInvestment"))
  (bind _output_get_2 (set `local.researchExpenses` _returnvalue_2))
  (`CMonthlyExpenseInvestment.Initialise` _output_get_2 (`local.researchBudget`) (`local.researchInvestmentLevels`))
  ;[1 1 1] Initialise the companyitself
  (`CCompany.InitialiseWithMultiplier` (`local.playerCompany`) 1000000 "/Game/Assets/ONNX-Models/netIncome_neural_net.netIncome_neural_net" "Data/scaling_data_information.json" 650 (`|MakeMap` "Marketing" (`local.marketingExpenses`) "ResearchAndDevelopment" (`local.researchExpenses`) :!type "ECompanyMonthyExpenseType Enum") 0.05 50 (make `SFinancialData` (`KismetMathLibrary.MakeDateTime` 2024 1 1) -12250000.0 12203000.0 287009000.0 1023961000.0 736952000.0 445297000.0 187.11 -20000000.0))
  ;[1 1 1] Set gameplay balance properties for the company
  ;;[1 1 1] Cap the net income change
  (`CCompany.SetNetIncomeMonthlyChangeCap` (`local.playerCompany`) 0.1 100000.0 true)
  ;;[1 1 1] Set a handicap for the net income
  (`CCompany.SetNetIncomeHandicapAmount` (`local.playerCompany`) 24000000)
  ;;[1 1 1] Cap the max stock value (marketing bonus effect)
  (`CCompany.SetMaxStockValue` (`local.playerCompany`) 650.0)
  ;;[1 1 1] Reduce the marketing bonus when the net income is negative
  (`CCompany.SetNegativeNetIncomeMarketingBonusRate` (`local.playerCompany`) 0.5))

(fn `UserConstructionScript`)