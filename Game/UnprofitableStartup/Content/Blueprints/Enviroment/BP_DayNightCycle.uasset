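; Day-night cycle Blueprint that rotates a sun light and drives sun and skylight intensity.
; Tick pitches the sun at the current cycle speed, refreshes the sky sphere and switches between day and night speeds within sunset and sunrise pitch windows.
; DoOnce gates trigger one timeline, played forward for nightfall and reversed for daybreak, to blend both light intensities.
; BeginPlay applies the daytime settings.
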(event `self.ReceiveBeginPlay`
  ;[1 1 1] Comment
  (`self.SetLightSettings` (`self.m_dayCycleSpeed`) (`self.m_daySunLightIntensity`) (`self.m_daySkyLightIntensity`)))

(event `self.ReceiveTick`
  (params (DeltaSeconds :type "Float (single-precision)"))
  (bind (_returnvalue_roll _returnvalue_pitch) (`KismetMathLibrary.BreakRotator` (`self.K2_GetActorRotation` (`self.m_sunLight`))))
  ;[1 1 1] Rotate the sun
  (`self.K2_AddActorLocalRotation` (`self.m_sunLight`) (`KismetMathLibrary.MakeRotator` 0.0 (* DeltaSeconds (`self.m_currentSpeedCycle`))) false false)
  (`/Engine/EngineSky/BP_Sky_Sphere.UpdateSunDirection` (`self.m_skySphere`))
  (if (and (< _returnvalue_pitch 75.0) (> _returnvalue_pitch 65.0))
    ;[1 1 1] Night
    (set `self.m_currentSpeedCycle` (`self.m_nightCycleSpeed`))
    (`/Engine/EditorBlueprintResources/StandardMacros.DoOnce` false :!label _label
      (:`Completed`
        ;[1 1 1] Animate sunrise and sunset
        (bind (_direction _cycletrack) (`Timeline|DayNightCycleTimeline` :!label _label_2)
          (:`Update`
            ;[1 1 1] Set lights intensity
            (`LightComponent.SetIntensity` (`Light.LightComponent` (`self.m_sunLight`)) (`KismetMathLibrary.Lerp` (`self.m_daySunLightIntensity`) (`self.m_nightSunLightIntensity`) _cycletrack))
            (`SkyLightComponent.SetIntensity` (`SkyLight.LightComponent` (`self.m_skyLight`)) (`KismetMathLibrary.Lerp` (`self.m_daySkyLightIntensity`) (`self.m_nightSkyLightIntensity`) _cycletrack)))
          (:`Finished`
            (`|ExecutionSequence`
              (:`then_0`
                (goto _label :!via `Reset`))
              (:`then_1`
                (goto _label_3 :!via `Reset`)))))))
    (elif (and (< _returnvalue_pitch 0.0) (> _returnvalue_pitch -15.0))
      ;[1 1 1] Day
      (set `self.m_currentSpeedCycle` (`self.m_dayCycleSpeed`))
      (`/Engine/EditorBlueprintResources/StandardMacros.DoOnce` false :!label _label_3
        (:`Completed`
          (goto _label_2 :!via `Reverse`))))))

(fn `SetLightSettings`
  (params (aRotationSpeed :type "Float (double-precision)") (aSunLightIntensity :type "Float (double-precision)") (aSkylightIntensity :type "Float (double-precision)"))
  (set `self.m_currentSpeedCycle` aRotationSpeed)
  (`LightComponent.SetIntensity` (`Light.LightComponent` (`self.m_sunLight`)) aSunLightIntensity)
  (`SkyLightComponent.SetIntensity` (`SkyLight.LightComponent` (`self.m_skyLight`)) aSkylightIntensity))

(fn `UserConstructionScript`)